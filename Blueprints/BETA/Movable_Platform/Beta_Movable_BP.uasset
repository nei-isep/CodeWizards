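; Beta movable platform that moves its static mesh between start and end point components, with an optional child jump pad.
; On BeginPlay, a bool activates the jump pad child component or deactivates the Beta_Jump_Pad_BG actor, then plays a timeline.
; The timeline lerps the mesh's world location between the two points.
; Timer-driven MoveTo and MoveComponentTo alternatives remain unconnected, and debug prints are left in.
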(event `self.ReceiveBeginPlay`
  (bind _childactor (`self.ChildActor`))
  (if (`self.b_should_have_jump_pad`)
    (`ActorComponent.SetActive` _childactor true true)
    (`KismetSystemLibrary.PrintString` "Hello")
    (bind (_direction _newtrack_0) (`Timeline|Timeline_0` :!label _label)
      (:`Update`
        (`SceneComponent.K2_SetWorldLocation` (`self.StaticMesh`) (`KismetMathLibrary.VLerp` (`SceneComponent.K2_GetComponentLocation` (`self.Starting_Point`)) (`SceneComponent.K2_GetComponentLocation` (`self.Endpoint`)) _newtrack_0) false false))
      (:`Finished`
        (`KismetSystemLibrary.PrintString` "Finished")))
    (else
      (bind _asbeta_jump_pad_bg (cast `/Game/Blueprints/BETA/JumpPad/Beta_Jump_Pad_BG` (`ChildActorComponent.ChildActor` _childactor)))
      (`/Game/Blueprints/BETA/JumpPad/Beta_Jump_Pad_BG.Set_Active` _asbeta_jump_pad_bg false)
      (goto _label))))

(fn `Move_To`
  (bind _output_get (set `self.Time passed` (+ (`GameplayStatics.GetWorldDeltaSeconds`) (`self.Time passed`))))
  (`KismetSystemLibrary.PrintString` (`KismetStringLibrary.Conv_DoubleToString` _output_get))
  (`SceneComponent.K2_SetWorldLocation` (`self.StaticMesh`) (`KismetMathLibrary.VLerp` (`SceneComponent.K2_GetComponentLocation` (`self.Starting_Point`)) (`SceneComponent.K2_GetComponentLocation` (`self.Endpoint`)) _output_get) false false)
  (if (>= _output_get 1.0)
    _))

(fn `UserConstructionScript`)